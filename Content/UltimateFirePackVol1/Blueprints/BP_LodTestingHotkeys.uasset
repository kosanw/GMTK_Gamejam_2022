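; Debug hotkey actor for testing Niagara fire LODs across four fire sizes and preset viewing distances.
; Numpad keys activate or deactivate the child-actor fires by size or toggle Niagara stat displays, with NumPad 9 bound to both.
; Number-row keys set WhichDistance; a shared sequence, also run after size changes, moves all fires to a fixed world Y up to 1 km out, using the tiny fire's X and Z.
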(event `self.ReceiveBeginPlay`
  (`self.EnableInput` (`GameplayStatics.GetPlayerController` 0)))

(event `Key|NumPadSeven`
  (params (Key :type "Key Structure"))
  (:`Pressed`
    (`KismetSystemLibrary.ExecuteConsoleCommand` "stat NiagaraEmitters" (`GameplayStatics.GetPlayerController` 0))))

(event `Key|NumPadEight`
  (params (Key :type "Key Structure"))
  (:`Pressed`
    (`KismetSystemLibrary.ExecuteConsoleCommand` "stat NiagaraSystems" (`GameplayStatics.GetPlayerController` 0))))

(event `Key|NumPadNine`
  (params (Key :type "Key Structure"))
  (:`Pressed`
    (`KismetSystemLibrary.ExecuteConsoleCommand` "stat Niagara" (`GameplayStatics.GetPlayerController` 0))))

(event `Key|NumPadFive`
  (params (Key :type "Key Structure"))
  (:`Pressed`
    (`KismetSystemLibrary.ExecuteConsoleCommand` "stat NiagaraSystemCounts" (`GameplayStatics.GetPlayerController` 0))))

(event `Key|NumPadSix`
  (params (Key :type "Key Structure"))
  (:`Pressed`
    (`KismetSystemLibrary.ExecuteConsoleCommand` "stat NiagaraOverview" (`GameplayStatics.GetPlayerController` 0))))

(event `Key|One`
  (params (Key :type "Key Structure"))
  (bind _bp_tinyfire___moving (`self.BP_TinyFire - moving`))
  (bind _bp_tinyfire___moving_2 (`self.BP_TinyFire - moving`))
  (bind _bp_tinyfire___moving_3 (`self.BP_TinyFire - moving`))
  (bind _bp_tinyfire___moving_4 (`self.BP_TinyFire - moving`))
  (bind _bp_tinyfire___moving_5 (`self.BP_TinyFire - moving`))
  (bind _bp_tinyfire___moving_6 (`self.BP_TinyFire - moving`))
  (bind _bp_tinyfire___moving_7 (`self.BP_TinyFire - moving`))
  (bind _bp_tinyfire___moving_8 (`self.BP_TinyFire - moving`))
  (bind _bp_tinyfire___moving_9 (`self.BP_TinyFire - moving`))
  (bind _bp_tinyfire___moving_10 (`self.BP_TinyFire - moving`))
  (bind _returnvalue (`KismetMathLibrary.MakeVector` (.x (`SceneComponent.K2_GetComponentLocation` _bp_tinyfire___moving_10)) -100000.0 (.z (`SceneComponent.K2_GetComponentLocation` _bp_tinyfire___moving_10))))
  (bind _returnvalue_2 (`KismetMathLibrary.MakeVector` (.x (`SceneComponent.K2_GetComponentLocation` _bp_tinyfire___moving_7)) -500.0 (.z (`SceneComponent.K2_GetComponentLocation` _bp_tinyfire___moving_7))))
  (bind _returnvalue_3 (`KismetMathLibrary.MakeVector` (.x (`SceneComponent.K2_GetComponentLocation` _bp_tinyfire___moving_9)) -100.0 (.z (`SceneComponent.K2_GetComponentLocation` _bp_tinyfire___moving_9))))
  (bind _returnvalue_4 (`KismetMathLibrary.MakeVector` (.x (`SceneComponent.K2_GetComponentLocation` _bp_tinyfire___moving_8)) 0.0 (.z (`SceneComponent.K2_GetComponentLocation` _bp_tinyfire___moving_8))))
  (bind _returnvalue_5 (`KismetMathLibrary.MakeVector` (.x (`SceneComponent.K2_GetComponentLocation` _bp_tinyfire___moving_3)) -5000.0 (.z (`SceneComponent.K2_GetComponentLocation` _bp_tinyfire___moving_3))))
  (bind _returnvalue_6 (`KismetMathLibrary.MakeVector` (.x (`SceneComponent.K2_GetComponentLocation` _bp_tinyfire___moving_4)) -10000.0 (.z (`SceneComponent.K2_GetComponentLocation` _bp_tinyfire___moving_4))))
  (bind _returnvalue_7 (`KismetMathLibrary.MakeVector` (.x (`SceneComponent.K2_GetComponentLocation` _bp_tinyfire___moving)) -1000.0 (.z (`SceneComponent.K2_GetComponentLocation` _bp_tinyfire___moving))))
  (bind _returnvalue_8 (`KismetMathLibrary.MakeVector` (.x (`SceneComponent.K2_GetComponentLocation` _bp_tinyfire___moving_5)) -25000.0 (.z (`SceneComponent.K2_GetComponentLocation` _bp_tinyfire___moving_5))))
  (bind _returnvalue_9 (`KismetMathLibrary.MakeVector` (.x (`SceneComponent.K2_GetComponentLocation` _bp_tinyfire___moving_6)) -50000.0 (.z (`SceneComponent.K2_GetComponentLocation` _bp_tinyfire___moving_6))))
  (bind _returnvalue_10 (`KismetMathLibrary.MakeVector` (.x (`SceneComponent.K2_GetComponentLocation` _bp_tinyfire___moving_2)) -2500.0 (.z (`SceneComponent.K2_GetComponentLocation` _bp_tinyfire___moving_2))))
  ;[1 1 1] Keys change variables, Then run Activates/Deactivates
  (:`Pressed`
    (`KismetSystemLibrary.PrintString` "Number Row 1 Pressed! (Distance: Self)" true true (struct :`G` 0.66 :`B` 1.0 :`A` 1.0) 10.0)
    (set `self.WhichDistance` 1)
    ;[1 1 1] Distance Switches
    (`|ExecutionSequence` :!label _label
      (:`then_0`
        ;;[1 1 1] Distance: Self
        (if (== 1 (`self.WhichDistance`))
          (`SceneComponent.K2_SetWorldLocation` _bp_tinyfire___moving_8 _returnvalue_4 false false)
          (`SceneComponent.K2_SetWorldLocation` (`self.BP_SmallFire - moving`) _returnvalue_4 false false)
          (`SceneComponent.K2_SetWorldLocation` (`self.BP_MediumFire - moving`) _returnvalue_4 false false)
          (`SceneComponent.K2_SetWorldLocation` (`self.BP_LargeFire - moving`) _returnvalue_4 false false)))
      (:`then_1`
        ;;[1 1 1] Distance: 1 Meter
        (if (== 2 (`self.WhichDistance`))
          (`SceneComponent.K2_SetWorldLocation` _bp_tinyfire___moving_9 _returnvalue_3 false false)
          (`SceneComponent.K2_SetWorldLocation` (`self.BP_SmallFire - moving`) _returnvalue_3 false false)
          (`SceneComponent.K2_SetWorldLocation` (`self.BP_MediumFire - moving`) _returnvalue_3 false false)
          (`SceneComponent.K2_SetWorldLocation` (`self.BP_LargeFire - moving`) _returnvalue_3 false false)))
      (:`then_2`
        ;;[1 1 1] Distance: 5 Meters
        (if (== 3 (`self.WhichDistance`))
          (`SceneComponent.K2_SetWorldLocation` _bp_tinyfire___moving_7 _returnvalue_2 false false)
          (`SceneComponent.K2_SetWorldLocation` (`self.BP_SmallFire - moving`) _returnvalue_2 false false)
          (`SceneComponent.K2_SetWorldLocation` (`self.BP_MediumFire - moving`) _returnvalue_2 false false)
          (`SceneComponent.K2_SetWorldLocation` (`self.BP_LargeFire - moving`) _returnvalue_2 false false)))
      (:`then_3`
        ;;[1 1 1] Distance: 10 Meters
        (if (== 4 (`self.WhichDistance`))
          (`SceneComponent.K2_SetWorldLocation` _bp_tinyfire___moving _returnvalue_7 false false)
          (`SceneComponent.K2_SetWorldLocation` (`self.BP_SmallFire - moving`) _returnvalue_7 false false)
          (`SceneComponent.K2_SetWorldLocation` (`self.BP_MediumFire - moving`) _returnvalue_7 false false)
          (`SceneComponent.K2_SetWorldLocation` (`self.BP_LargeFire - moving`) _returnvalue_7 false false)))
      (:`then_4`
        ;;[1 1 1] Distance 25 Meters
        (if (== 5 (`self.WhichDistance`))
          (`SceneComponent.K2_SetWorldLocation` _bp_tinyfire___moving_2 _returnvalue_10 false false)
          (`SceneComponent.K2_SetWorldLocation` (`self.BP_SmallFire - moving`) _returnvalue_10 false false)
          (`SceneComponent.K2_SetWorldLocation` (`self.BP_MediumFire - moving`) _returnvalue_10 false false)
          (`SceneComponent.K2_SetWorldLocation` (`self.BP_LargeFire - moving`) _returnvalue_10 false false)))
      (:`then_5`
        ;;[1 1 1] Distance: 50 Meters
        (if (== 6 (`self.WhichDistance`))
          (`SceneComponent.K2_SetWorldLocation` _bp_tinyfire___moving_3 _returnvalue_5 false false)
          (`SceneComponent.K2_SetWorldLocation` (`self.BP_SmallFire - moving`) _returnvalue_5 false false)
          (`SceneComponent.K2_SetWorldLocation` (`self.BP_MediumFire - moving`) _returnvalue_5 false false)
          (`SceneComponent.K2_SetWorldLocation` (`self.BP_LargeFire - moving`) _returnvalue_5 false false)))
      (:`then_6`
        ;;[1 1 1] Distance: 100 Meters
        (if (== 7 (`self.WhichDistance`))
          (`SceneComponent.K2_SetWorldLocation` _bp_tinyfire___moving_4 _returnvalue_6 false false)
          (`SceneComponent.K2_SetWorldLocation` (`self.BP_SmallFire - moving`) _returnvalue_6 false false)
          (`SceneComponent.K2_SetWorldLocation` (`self.BP_MediumFire - moving`) _returnvalue_6 false false)
          (`SceneComponent.K2_SetWorldLocation` (`self.BP_LargeFire - moving`) _returnvalue_6 false false)))
      (:`then_7`
        ;;[1 1 1] Distance: 250 Meters
        (if (== 8 (`self.WhichDistance`))
          (`SceneComponent.K2_SetWorldLocation` _bp_tinyfire___moving_5 _returnvalue_8 false false)
          (`SceneComponent.K2_SetWorldLocation` (`self.BP_SmallFire - moving`) _returnvalue_8 false false)
          (`SceneComponent.K2_SetWorldLocation` (`self.BP_MediumFire - moving`) _returnvalue_8 false false)
          (`SceneComponent.K2_SetWorldLocation` (`self.BP_LargeFire - moving`) _returnvalue_8 false false)))
      (:`then_8`
        ;;[1 1 1] Distance: 500 Meters
        (if (== 9 (`self.WhichDistance`))
          (`SceneComponent.K2_SetWorldLocation` _bp_tinyfire___moving_6 _returnvalue_9 false false)
          (`SceneComponent.K2_SetWorldLocation` (`self.BP_SmallFire - moving`) _returnvalue_9 false false)
          (`SceneComponent.K2_SetWorldLocation` (`self.BP_MediumFire - moving`) _returnvalue_9 false false)
          (`SceneComponent.K2_SetWorldLocation` (`self.BP_LargeFire - moving`) _returnvalue_9 false false)))
      (:`then_9`
        ;;[1 1 1] Distance: 1,00 Meters
        (if (== 10 (`self.WhichDistance`))
          (`SceneComponent.K2_SetWorldLocation` _bp_tinyfire___moving_10 _returnvalue false false)
          (`SceneComponent.K2_SetWorldLocation` (`self.BP_SmallFire - moving`) _returnvalue false false)
          (`SceneComponent.K2_SetWorldLocation` (`self.BP_MediumFire - moving`) _returnvalue false false)
          (`SceneComponent.K2_SetWorldLocation` (`self.BP_LargeFire - moving`) _returnvalue false false))))))

(event `Key|NumPadOne`
  (params (Key :type "Key Structure"))
  ;[1 1 1] Keys change variables, Then run Activates/Deactivates
  (:`Pressed`
    (`KismetSystemLibrary.PrintString` "Number Pad 1 Pressed! (Size: Tiny)" true true (struct :`G` 0.66 :`B` 1.0 :`A` 1.0) 10.0)
    (set `self.WhichSize` 1)
    (bind _asbp_tiny_fire (cast `/Game/UltimateFirePackVol1/Particles/Fire/Niagara/FireTiny/BP_TinyFire` (`ChildActorComponent.ChildActor` (`self.BP_TinyFire - moving`))))
    (`ActorComponent.Activate` (`/Game/UltimateFirePackVol1/Particles/Fire/Niagara/FireTiny/BP_TinyFire.Niagara` _asbp_tiny_fire) false)
    (bind _asbp_small_fire (cast `/Game/UltimateFirePackVol1/Particles/Fire/Niagara/FireSmall/BP_SmallFire` (`ChildActorComponent.ChildActor` (`self.BP_SmallFire - moving`))))
    (`ActorComponent.Deactivate` (`/Game/UltimateFirePackVol1/Particles/Fire/Niagara/FireSmall/BP_SmallFire.Niagara` _asbp_small_fire))
    (bind _asbp_medium_fire (cast `/Game/UltimateFirePackVol1/Particles/Fire/Niagara/FireMedium/BP_MediumFire` (`ChildActorComponent.ChildActor` (`self.BP_MediumFire - moving`))))
    (`ActorComponent.Deactivate` (`/Game/UltimateFirePackVol1/Particles/Fire/Niagara/FireMedium/BP_MediumFire.Niagara` _asbp_medium_fire))
    (bind _asbp_large_fire (cast `/Game/UltimateFirePackVol1/Particles/Fire/Niagara/FireLarge/BP_LargeFire` (`ChildActorComponent.ChildActor` (`self.BP_LargeFire - moving`))))
    (`ActorComponent.Deactivate` (`/Game/UltimateFirePackVol1/Particles/Fire/Niagara/FireLarge/BP_LargeFire.Niagara` _asbp_large_fire))
    (goto _label)))

(event `Key|Two`
  (params (Key :type "Key Structure"))
  ;[1 1 1] Keys change variables, Then run Activates/Deactivates
  (:`Pressed`
    (`KismetSystemLibrary.PrintString` "Number Row 2 Pressed! (Distance: 1 Meter)" true true (struct :`G` 0.66 :`B` 1.0 :`A` 1.0) 10.0)
    (set `self.WhichDistance` 2)
    (goto _label)))

(event `Key|NumPadTwo`
  (params (Key :type "Key Structure"))
  ;[1 1 1] Keys change variables, Then run Activates/Deactivates
  (:`Pressed`
    (`KismetSystemLibrary.PrintString` "Number Pad 1 Pressed! (Size: Small)" true true (struct :`G` 0.66 :`B` 1.0 :`A` 1.0) 10.0)
    (set `self.WhichSize` 2)
    (bind _asbp_small_fire (cast `/Game/UltimateFirePackVol1/Particles/Fire/Niagara/FireSmall/BP_SmallFire` (`ChildActorComponent.ChildActor` (`self.BP_SmallFire - moving`))))
    (`ActorComponent.Activate` (`/Game/UltimateFirePackVol1/Particles/Fire/Niagara/FireSmall/BP_SmallFire.Niagara` _asbp_small_fire) false)
    (bind _asbp_tiny_fire (cast `/Game/UltimateFirePackVol1/Particles/Fire/Niagara/FireTiny/BP_TinyFire` (`ChildActorComponent.ChildActor` (`self.BP_TinyFire - moving`))))
    (`ActorComponent.Deactivate` (`/Game/UltimateFirePackVol1/Particles/Fire/Niagara/FireTiny/BP_TinyFire.Niagara` _asbp_tiny_fire))
    (bind _asbp_medium_fire (cast `/Game/UltimateFirePackVol1/Particles/Fire/Niagara/FireMedium/BP_MediumFire` (`ChildActorComponent.ChildActor` (`self.BP_MediumFire - moving`))))
    (`ActorComponent.Deactivate` (`/Game/UltimateFirePackVol1/Particles/Fire/Niagara/FireMedium/BP_MediumFire.Niagara` _asbp_medium_fire))
    (bind _asbp_large_fire (cast `/Game/UltimateFirePackVol1/Particles/Fire/Niagara/FireLarge/BP_LargeFire` (`ChildActorComponent.ChildActor` (`self.BP_LargeFire - moving`))))
    (`ActorComponent.Deactivate` (`/Game/UltimateFirePackVol1/Particles/Fire/Niagara/FireLarge/BP_LargeFire.Niagara` _asbp_large_fire))
    (goto _label)))

(event `Key|Three`
  (params (Key :type "Key Structure"))
  ;[1 1 1] Keys change variables, Then run Activates/Deactivates
  (:`Pressed`
    (`KismetSystemLibrary.PrintString` "Number Row 3 Pressed! (Distance: 5 Meters)" true true (struct :`G` 0.66 :`B` 1.0 :`A` 1.0) 10.0)
    (set `self.WhichDistance` 3)
    (goto _label)))

(event `Key|NumPadThree`
  (params (Key :type "Key Structure"))
  ;[1 1 1] Keys change variables, Then run Activates/Deactivates
  (:`Pressed`
    (`KismetSystemLibrary.PrintString` "Number Pad 1 Pressed! (Size: Medium)" true true (struct :`G` 0.66 :`B` 1.0 :`A` 1.0) 10.0)
    (set `self.WhichSize` 3)
    (bind _asbp_medium_fire (cast `/Game/UltimateFirePackVol1/Particles/Fire/Niagara/FireMedium/BP_MediumFire` (`ChildActorComponent.ChildActor` (`self.BP_MediumFire - moving`))))
    (`ActorComponent.Activate` (`/Game/UltimateFirePackVol1/Particles/Fire/Niagara/FireMedium/BP_MediumFire.Niagara` _asbp_medium_fire) false)
    (bind _asbp_tiny_fire (cast `/Game/UltimateFirePackVol1/Particles/Fire/Niagara/FireTiny/BP_TinyFire` (`ChildActorComponent.ChildActor` (`self.BP_TinyFire - moving`))))
    (`ActorComponent.Deactivate` (`/Game/UltimateFirePackVol1/Particles/Fire/Niagara/FireTiny/BP_TinyFire.Niagara` _asbp_tiny_fire))
    (bind _asbp_small_fire (cast `/Game/UltimateFirePackVol1/Particles/Fire/Niagara/FireSmall/BP_SmallFire` (`ChildActorComponent.ChildActor` (`self.BP_SmallFire - moving`))))
    (`ActorComponent.Deactivate` (`/Game/UltimateFirePackVol1/Particles/Fire/Niagara/FireSmall/BP_SmallFire.Niagara` _asbp_small_fire))
    (bind _asbp_large_fire (cast `/Game/UltimateFirePackVol1/Particles/Fire/Niagara/FireLarge/BP_LargeFire` (`ChildActorComponent.ChildActor` (`self.BP_LargeFire - moving`))))
    (`ActorComponent.Deactivate` (`/Game/UltimateFirePackVol1/Particles/Fire/Niagara/FireLarge/BP_LargeFire.Niagara` _asbp_large_fire))
    (goto _label)))

(event `Key|Four`
  (params (Key :type "Key Structure"))
  ;[1 1 1] Keys change variables, Then run Activates/Deactivates
  (:`Pressed`
    (`KismetSystemLibrary.PrintString` "Number Row 4 Pressed! (Distance: 10 Meters)" true true (struct :`G` 0.66 :`B` 1.0 :`A` 1.0) 10.0)
    (set `self.WhichDistance` 4)
    (goto _label)))

(event `Key|NumPadFour`
  (params (Key :type "Key Structure"))
  ;[1 1 1] Keys change variables, Then run Activates/Deactivates
  (:`Pressed`
    (`KismetSystemLibrary.PrintString` "Number Pad 1 Pressed! (Size: Large)" true true (struct :`G` 0.66 :`B` 1.0 :`A` 1.0) 10.0)
    (set `self.WhichSize` 4)
    (bind _asbp_large_fire (cast `/Game/UltimateFirePackVol1/Particles/Fire/Niagara/FireLarge/BP_LargeFire` (`ChildActorComponent.ChildActor` (`self.BP_LargeFire - moving`))))
    (`ActorComponent.Activate` (`/Game/UltimateFirePackVol1/Particles/Fire/Niagara/FireLarge/BP_LargeFire.Niagara` _asbp_large_fire) false)
    (bind _asbp_tiny_fire (cast `/Game/UltimateFirePackVol1/Particles/Fire/Niagara/FireTiny/BP_TinyFire` (`ChildActorComponent.ChildActor` (`self.BP_TinyFire - moving`))))
    (`ActorComponent.Deactivate` (`/Game/UltimateFirePackVol1/Particles/Fire/Niagara/FireTiny/BP_TinyFire.Niagara` _asbp_tiny_fire))
    (bind _asbp_small_fire (cast `/Game/UltimateFirePackVol1/Particles/Fire/Niagara/FireSmall/BP_SmallFire` (`ChildActorComponent.ChildActor` (`self.BP_SmallFire - moving`))))
    (`ActorComponent.Deactivate` (`/Game/UltimateFirePackVol1/Particles/Fire/Niagara/FireSmall/BP_SmallFire.Niagara` _asbp_small_fire))
    (bind _asbp_medium_fire (cast `/Game/UltimateFirePackVol1/Particles/Fire/Niagara/FireMedium/BP_MediumFire` (`ChildActorComponent.ChildActor` (`self.BP_MediumFire - moving`))))
    (`ActorComponent.Deactivate` (`/Game/UltimateFirePackVol1/Particles/Fire/Niagara/FireMedium/BP_MediumFire.Niagara` _asbp_medium_fire))
    (goto _label)))

(event `Key|Five`
  (params (Key :type "Key Structure"))
  ;[1 1 1] Keys change variables, Then run Activates/Deactivates
  (:`Pressed`
    (`KismetSystemLibrary.PrintString` "Number Row 5 Pressed! (Distance: 25 Meters)" true true (struct :`G` 0.66 :`B` 1.0 :`A` 1.0) 10.0)
    (set `self.WhichDistance` 5)
    (goto _label)))

(event `Key|Six`
  (params (Key :type "Key Structure"))
  ;[1 1 1] Keys change variables, Then run Activates/Deactivates
  (:`Pressed`
    (`KismetSystemLibrary.PrintString` "Number Row 6 Pressed! (Distance: 50 Meters)" true true (struct :`G` 0.66 :`B` 1.0 :`A` 1.0) 10.0)
    (set `self.WhichDistance` 6)
    (goto _label)))

(event `Key|Seven`
  (params (Key :type "Key Structure"))
  ;[1 1 1] Keys change variables, Then run Activates/Deactivates
  (:`Pressed`
    (`KismetSystemLibrary.PrintString` "Number Row 7 Pressed! (Distance: 100 Meters)" true true (struct :`G` 0.66 :`B` 1.0 :`A` 1.0) 10.0)
    (set `self.WhichDistance` 7)
    (goto _label)))

(event `Key|Eight`
  (params (Key :type "Key Structure"))
  ;[1 1 1] Keys change variables, Then run Activates/Deactivates
  (:`Pressed`
    (`KismetSystemLibrary.PrintString` "Number Row 8 Pressed! (Distance: 250 Meters)" true true (struct :`G` 0.66 :`B` 1.0 :`A` 1.0) 10.0)
    (set `self.WhichDistance` 8)
    (goto _label)))

(event `Key|Nine`
  (params (Key :type "Key Structure"))
  ;[1 1 1] Keys change variables, Then run Activates/Deactivates
  (:`Pressed`
    (`KismetSystemLibrary.PrintString` "Number Row 9 Pressed! (Distance: 500 Meters)" true true (struct :`G` 0.66 :`B` 1.0 :`A` 1.0) 10.0)
    (set `self.WhichDistance` 9)
    (goto _label)))

(event `Key|Zero`
  (params (Key :type "Key Structure"))
  ;[1 1 1] Keys change variables, Then run Activates/Deactivates
  (:`Pressed`
    (`KismetSystemLibrary.PrintString` "Number Row 0 Pressed! (Distance: 1,000 Meters)" true true (struct :`G` 0.66 :`B` 1.0 :`A` 1.0) 10.0)
    (set `self.WhichDistance` 10)
    (goto _label)))

(event `Key|NumPadNine`
  (params (Key :type "Key Structure"))
  ;[1 1 1] Keys change variables, Then run Activates/Deactivates
  (:`Pressed`
    (`KismetSystemLibrary.PrintString` "Number Pad 9 Pressed! (Size: All)" true true (struct :`G` 0.66 :`B` 1.0 :`A` 1.0) 10.0)
    (set `self.WhichSize` 0)
    (bind _asbp_tiny_fire (cast `/Game/UltimateFirePackVol1/Particles/Fire/Niagara/FireTiny/BP_TinyFire` (`ChildActorComponent.ChildActor` (`self.BP_TinyFire - moving`))))
    (`ActorComponent.Activate` (`/Game/UltimateFirePackVol1/Particles/Fire/Niagara/FireTiny/BP_TinyFire.Niagara` _asbp_tiny_fire) false)
    (bind _asbp_small_fire (cast `/Game/UltimateFirePackVol1/Particles/Fire/Niagara/FireSmall/BP_SmallFire` (`ChildActorComponent.ChildActor` (`self.BP_SmallFire - moving`))))
    (`ActorComponent.Activate` (`/Game/UltimateFirePackVol1/Particles/Fire/Niagara/FireSmall/BP_SmallFire.Niagara` _asbp_small_fire) false)
    (bind _asbp_medium_fire (cast `/Game/UltimateFirePackVol1/Particles/Fire/Niagara/FireMedium/BP_MediumFire` (`ChildActorComponent.ChildActor` (`self.BP_MediumFire - moving`))))
    (`ActorComponent.Activate` (`/Game/UltimateFirePackVol1/Particles/Fire/Niagara/FireMedium/BP_MediumFire.Niagara` _asbp_medium_fire) false)
    (bind _asbp_large_fire (cast `/Game/UltimateFirePackVol1/Particles/Fire/Niagara/FireLarge/BP_LargeFire` (`ChildActorComponent.ChildActor` (`self.BP_LargeFire - moving`))))
    (`ActorComponent.Activate` (`/Game/UltimateFirePackVol1/Particles/Fire/Niagara/FireLarge/BP_LargeFire.Niagara` _asbp_large_fire) false)
    (goto _label)))

(event `Key|NumPadZero`
  (params (Key :type "Key Structure"))
  ;[1 1 1] Keys change variables, Then run Activates/Deactivates
  (:`Pressed`
    (`KismetSystemLibrary.PrintString` "Number Pad 0 Pressed! (Size: None)" true true (struct :`G` 0.66 :`B` 1.0 :`A` 1.0) 10.0)
    (set `self.WhichSize` 0)
    (bind _asbp_tiny_fire (cast `/Game/UltimateFirePackVol1/Particles/Fire/Niagara/FireTiny/BP_TinyFire` (`ChildActorComponent.ChildActor` (`self.BP_TinyFire - moving`))))
    (`ActorComponent.Deactivate` (`/Game/UltimateFirePackVol1/Particles/Fire/Niagara/FireTiny/BP_TinyFire.Niagara` _asbp_tiny_fire))
    (bind _asbp_small_fire (cast `/Game/UltimateFirePackVol1/Particles/Fire/Niagara/FireSmall/BP_SmallFire` (`ChildActorComponent.ChildActor` (`self.BP_SmallFire - moving`))))
    (`ActorComponent.Deactivate` (`/Game/UltimateFirePackVol1/Particles/Fire/Niagara/FireSmall/BP_SmallFire.Niagara` _asbp_small_fire))
    (bind _asbp_medium_fire (cast `/Game/UltimateFirePackVol1/Particles/Fire/Niagara/FireMedium/BP_MediumFire` (`ChildActorComponent.ChildActor` (`self.BP_MediumFire - moving`))))
    (`ActorComponent.Deactivate` (`/Game/UltimateFirePackVol1/Particles/Fire/Niagara/FireMedium/BP_MediumFire.Niagara` _asbp_medium_fire))
    (bind _asbp_large_fire (cast `/Game/UltimateFirePackVol1/Particles/Fire/Niagara/FireLarge/BP_LargeFire` (`ChildActorComponent.ChildActor` (`self.BP_LargeFire - moving`))))
    (`ActorComponent.Deactivate` (`/Game/UltimateFirePackVol1/Particles/Fire/Niagara/FireLarge/BP_LargeFire.Niagara` _asbp_large_fire))
    (goto _label)))

(fn `UserConstructionScript`)